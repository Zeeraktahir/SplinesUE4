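; Spline-based measuring line actor that stretches from its own location to the surface point under the mouse cursor while the player is drawing.
; On BeginPlay it adds a spline mesh along the spline, then a 0.1-second Delay loop moves the end point and mesh until the player controller's IsDrawing turns false.
; Each pass also updates text renders showing length in centimetres and planar angle in degrees.
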(event EventBeginPlay
  (bind _returnvalue (Transformation|GetActorLocation))
  (bind _spline (Variables|Default|GetSpline))
  (bind _spline_2 (Variables|Default|GetSpline))
  (bind _spline_3 (Variables|Default|GetSpline))
  (bind (_location _tangent) (Spline|GetLocationandTangentatSplinePoint _spline_2 1 "Local"))
  (bind (_location_2 _tangent_2) (Spline|GetLocationandTangentatSplinePoint _spline_3 0 "Local"))
  (Development|ExecuteConsoleCommand "show splines" 0)
  (bind _returnvalue_2 (AddComponent|AddSplineMeshComponent false))
  (bind _output_get (Variables|Default|SetMeshArc _returnvalue_2))
  (SplineMesh|SetForwardAxis _output_get "Z" true)
  (Transformation|AttachComponentToComponent (Variables|Default|GetMeshArc) (Variables|Default|GetSpline) "None" "KeepRelative" "KeepRelative" "KeepRelative" true)
  (bind _asbp_player_controller (Utilities|Casting|CastToBP_PlayerController (Game|GetPlayerController 0)))
  (Variables|Default|SetPlayerControllerRef _asbp_player_controller)
  (Spline|SetLocationatSplinePoint _spline 0 _returnvalue "World" true)
  (Spline|SetLocationatSplinePoint _spline 1 (.location (.HitResult (Game|Player|GetHitResultUnderCursorbyChannel (Variables|Default|GetPlayerControllerRef) "TraceTypeQuery1" true))) "World" true :!label _label)
  (SplineMesh|SetStartandEnd (Variables|Default|GetMeshArc) _location_2 _tangent_2 _location _tangent true :!class /Script/Engine.SplineMeshComponent)
  (Rendering|Components|TextRender|SetText (Variables|Default|GetTextRender) (Utilities|Text|ToText(String) (Utilities|String|Append (Utilities|String|ToString(Text) (Utilities|Text|ToText(Float) (/ (Spline|GetSplineLength (Variables|Default|GetSpline)) 1e+01) "HalfToEven" false true 1 324 0 1)) " cm")))
  (Rendering|Components|TextRender|SetText (Variables|Default|GetAngle) (Utilities|Text|ToText(String) (Utilities|String|Append (Utilities|String|ToString(Text) (Utilities|Text|ToText(Float) (+ (Class|KismetMathLibrary|DegAtan2 (.X (Math|Vector|BreakVector (- _returnvalue (.location (.HitResult (Game|Player|GetHitResultUnderCursorbyChannel (Variables|Default|GetPlayerControllerRef) "TraceTypeQuery1" true)))))) (.Y (Math|Vector|BreakVector (- _returnvalue (.location (.HitResult (Game|Player|GetHitResultUnderCursorbyChannel (Variables|Default|GetPlayerControllerRef) "TraceTypeQuery1" true))))))) 1.8e+02) "HalfToEven" false true 1 324 0 1)) "°")))
  (Utilities|FlowControl|Delay 0.1)
  (if (Variables|/Game/Blueprints/BP_PlayerController.BP_PlayerController_C|GetIsDrawing (Variables|Default|GetPlayerControllerRef))
    (goto _label)))

(fn ConstructionScript)