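; PolyLine is a Blueprint that sets up a spline-based polyline with line and arc modes, apparently an unfinished drawing tool.
; BeginPlay enables spline display, caches the BP_PlayerController, and attaches a new Z-forward spline mesh to the Spline.
; It then enters an empty loop while IsDrawing is true.
; Two input actions switch PolyLineMode, but nothing here reads it or adds spline points.
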(event EventBeginPlay
  (Development|ExecuteConsoleCommand "show splines" 0)
  (bind _asbp_player_controller (Utilities|Casting|CastToBP_PlayerController (Game|GetPlayerController 0)))
  (Variables|Default|SetPlayerController _asbp_player_controller)
  (Utilities|Array|Clear (Variables|Default|GetMeshes))
  (bind _returnvalue (AddComponent|AddSplineMeshComponent false))
  (bind _returnvalue_2 (Utilities|Array|Add (Variables|Default|GetMeshes) _returnvalue))
  (SplineMesh|SetForwardAxis (Utilities|Array|Get(acopy) (Variables|Default|GetMeshes) _returnvalue_2) "Z" true)
  (Transformation|AttachComponentToComponent (Utilities|Array|Get(acopy) (Variables|Default|GetMeshes) _returnvalue_2) (Variables|Default|GetSpline) "None" "KeepRelative" "KeepRelative" "KeepRelative" true)
  (while (Variables|Default|GetIsDrawing)
    _))

(event EventTick
  (params (DeltaSeconds :type Float%20%28single-precision%29)))

(event Input|ActionEvents|InputActionPolyLine_Arc
  (params (Key :type Key%20Structure :default "None"))
  (:Pressed
    (Variables|Default|SetPolyLine_Mode "NewEnumerator1")))

(event Input|ActionEvents|InputActionPolyLine_Line
  (params (Key :type Key%20Structure :default "None"))
  (:Pressed
    (Variables|Default|SetPolyLine_Mode "NewEnumerator0")))

(fn ConstructionScript)