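; Player controller for a cursor-driven drawing tool with line, arc and polyline modes.
; It creates the UI on BeginPlay, shows the mouse cursor, and routes left clicks by the selected mode to spawn actors at the traced cursor hit.
; Boolean flags track two-click lines and three-click arcs, while polylines spawn an actor per click while drawing is active, until right-click clears that flag.
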(event EventBeginPlay
  (bind _returnvalue (UserInterface|CreateWidget "/Game/Blueprints/UI.UI_C"))
  (UserInterface|Viewport|AddtoViewport _returnvalue 0))

(event Input|ActionEvents|InputActionMouseClick
  (params (Key :type Key%20Structure :default "None"))
  (bind _hitresult (Game|Player|GetHitResultUnderCursorbyChannel "TraceTypeQuery1" true))
  (:Pressed
    (switch string (Variables|Default|GetModeSelected)
      (:Line
        (if (Variables|Default|GetIsDrawing)
          (Variables|Default|SetIsDrawing false)
          (else
            (Game|SpawnActorfromClass "/Game/Blueprints/Spline2.Spline2_C" (Math|Transform|MakeTransform (.location _hitresult) "0, 0, 0" "1,1,1") "AlwaysSpawn" 0 0)
            (Variables|Default|SetIsDrawing true))))
      (:Arc
        (if (Variables|Default|GetIsFirstClick)
          (if (Variables|Default|GetIsSecondClick)
            (Variables|Default|SetIsFirstClick false)
            (Variables|Default|SetIsSecondClick false)
            (else
              (Variables|Default|SetIsSecondClick true)))
          (else
            (Game|SpawnActorfromClass "/Game/Blueprints/SplineArc.SplineArc_C" (Math|Transform|MakeTransform (.location _hitresult) "0, 0, 0" "1,1,1") "AlwaysSpawn" 0 0)
            (Variables|Default|SetIsFirstClick true))))
      (:PolyLine
        (if (Variables|Default|GetPolyLine_Drawing)
          (Game|SpawnActorfromClass "/Game/Blueprints/PolyLine.PolyLine_C" (Math|Transform|MakeTransform (.location _hitresult) "0, 0, 0" "1,1,1") "AlwaysSpawn" 0 0))))))

(event Input|ActionEvents|InputActionRightClick
  (params (Key :type Key%20Structure :default "None"))
  (:Pressed
    (Variables|Default|SetPolyLine_Drawing false)))

(fn ConstructionScript
  (Variables|Default|SetbShowMouseCursor true))