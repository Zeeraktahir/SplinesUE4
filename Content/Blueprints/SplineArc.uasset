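; SplineArc is an interactive actor that draws a spline-mesh arc from its location to the cursor and labels its length.
; On BeginPlay, a Delay-driven polling loop moves the second spline point to the cursor trace hit, updating the mesh and text.
; When BP_PlayerController's IsSecondClick becomes true, it adds a third point and second mesh segment, tracking the cursor until that flag clears.
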(event EventBeginPlay
  (bind _spline (Variables|Default|GetSpline))
  (bind _spline_2 (Variables|Default|GetSpline))
  (bind _spline_3 (Variables|Default|GetSpline))
  (bind _spline_4 (Variables|Default|GetSpline))
  (bind _spline_5 (Variables|Default|GetSpline))
  (bind (_location _tangent) (Spline|GetLocationandTangentatSplinePoint _spline_3 0 "Local"))
  (bind (_location_2 _tangent_2) (Spline|GetLocationandTangentatSplinePoint _spline 1 "Local"))
  (bind (_location_3 _tangent_3) (Spline|GetLocationandTangentatSplinePoint _spline_2 2 "Local"))
  (bind (_location_4 _tangent_4) (Spline|GetLocationandTangentatSplinePoint _spline_4 1 "Local"))
  (bind (_location_5 _tangent_5) (Spline|GetLocationandTangentatSplinePoint _spline_5 0 "Local"))
  (Development|ExecuteConsoleCommand "show splines" 0)
  (bind _returnvalue (AddComponent|AddSplineMeshComponent false))
  (bind _output_get (Variables|Default|SetMesh1 _returnvalue))
  (SplineMesh|SetForwardAxis _output_get "Z" true)
  (Transformation|AttachComponentToComponent (Variables|Default|GetMesh1) (Variables|Default|GetSpline) "None" "KeepRelative" "KeepRelative" "KeepRelative" true)
  (bind _asbp_player_controller (Utilities|Casting|CastToBP_PlayerController (Game|GetPlayerController 0)))
  (Variables|Default|SetPlayerController _asbp_player_controller)
  (Spline|SetLocationatSplinePoint (Variables|Default|GetSpline) 0 (Transformation|GetActorLocation) "World" true)
  (Spline|SetLocationatSplinePoint _spline_3 1 (.location (.HitResult (Game|Player|GetHitResultUnderCursorbyChannel (Variables|Default|GetPlayerController) "TraceTypeQuery1" true))) "World" true :!label _label)
  (SplineMesh|SetStartandEnd (Variables|Default|GetMesh1) _location (Math|Vector|MakeVector (.x _tangent) (.y _tangent) (.z _tangent)) _location_4 (Math|Vector|MakeVector (.x _tangent_4) (.y _tangent_4) (.z _tangent_4)) true :!class /Script/Engine.SplineMeshComponent)
  (Rendering|Components|TextRender|SetText (Variables|Default|GetTextRender) (Utilities|Text|ToText(Float) (/ (Spline|GetSplineLength (Variables|Default|GetSpline)) 1e+01) "HalfToEven" false true 1 324 0 1))
  (Utilities|FlowControl|Delay 0.01)
  (if (Variables|/Game/Blueprints/BP_PlayerController.BP_PlayerController_C|GetIsSecondClick (Variables|Default|GetPlayerController))
    (Spline|AddSplinePoint (Variables|Default|GetSpline) (.location (.HitResult (Game|Player|GetHitResultUnderCursorbyChannel (Variables|Default|GetPlayerController) "TraceTypeQuery1" true))) "World" true)
    (bind _returnvalue_2 (AddComponent|AddSplineMeshComponent false))
    (SplineMesh|SetForwardAxis _returnvalue_2 "Z" true)
    (Spline|SetLocationatSplinePoint (Variables|Default|GetSpline) 2 (Math|Vector|MakeVector (.X (Math|Vector|BreakVector (.location (.HitResult (Game|Player|GetHitResultUnderCursorbyChannel (Variables|Default|GetPlayerController) "TraceTypeQuery1" true))))) (.Y (Math|Vector|BreakVector (.location (.HitResult (Game|Player|GetHitResultUnderCursorbyChannel (Variables|Default|GetPlayerController) "TraceTypeQuery1" true))))) (.Z (Math|Vector|BreakVector (.location (.HitResult (Game|Player|GetHitResultUnderCursorbyChannel (Variables|Default|GetPlayerController) "TraceTypeQuery1" true)))))) "World" true :!label _label_2)
    (SplineMesh|SetStartandEnd (Variables|Default|GetMesh1) _location_5 _tangent_5 _location_2 _tangent_2 true :!class /Script/Engine.SplineMeshComponent)
    (SplineMesh|SetStartandEnd _returnvalue_2 _location_2 _tangent_2 _location_3 _tangent_3 true :!class /Script/Engine.SplineMeshComponent)
    (Utilities|FlowControl|Delay 0.01)
    (Rendering|Components|TextRender|SetText (Variables|Default|GetTextRender) (Utilities|Text|ToText(Float) (/ (Spline|GetSplineLength (Variables|Default|GetSpline)) 1e+01) "HalfToEven" false true 1 324 0 1))
    (if (Variables|/Game/Blueprints/BP_PlayerController.BP_PlayerController_C|GetIsSecondClick (Variables|Default|GetPlayerController))
      (goto _label_2)
      (else
        (Development|PrintString "Done Arc")))
    (else
      (goto _label))))

(fn ConstructionScript)